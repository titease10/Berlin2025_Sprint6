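; Level 1 game mode that runs a level timer and keeps a persistent best time.
; Tick adds delta time to the timer while the chrono is active, and a helper formats times as minutes and zero-padded seconds.
; BeginPlay loads the best time from an SG_BestTimes save slot, using -1 when no save exists.
; An update function saves the current time when it is lower or no record is set.
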(event `self.ReceiveBeginPlay`
  (`self.Load Best Time`)
  (`KismetSystemLibrary.PrintString` (`KismetStringLibrary.Conv_DoubleToString` (`self.BestTime`))))

(event `self.ReceiveTick`
  (params (DeltaSeconds :type "Float (single-precision)"))
  ;[1 1 1] ADD (Chrono feature)
  (if (`self.bChronoActif`)
    (set `self.ChronoTemps` (+ (`self.ChronoTemps`) DeltaSeconds))))

(fn `Check And Update Best Time`
  (bind _chronotemps (`self.ChronoTemps`))
  (bind _besttime (`self.BestTime`))
  (if (or (< _chronotemps _besttime) (< _besttime 0.0))
    (set `self.BestTime` _chronotemps)
    (`self.Save Best Time`)))

(fn `Get Formatted Time`
  (params (Time :type "Float (double-precision)"))
  (returns (TimeFormated :type String))
  (bind (_days _hours _minutes _seconds) (`KismetMathLibrary.BreakTimespan` (`KismetMathLibrary.MakeTimespan2` 0 0 0 (`KismetMathLibrary.FTrunc` Time))))
  (if (< _seconds 10)
    (return (`KismetTextLibrary.Conv_TextToString` (`|FormatText` "{MM}:{SS}" _minutes (`KismetStringLibrary.Concat_StrStr` "0" (`KismetStringLibrary.Conv_IntToString` _seconds)))))
    (else
      (return (`KismetTextLibrary.Conv_TextToString` (`|FormatText` "{MM}:{SS}" _minutes _seconds))))))

(fn `Load Best Time`
  (bind _returnvalue (`GameplayStatics.DoesSaveGameExist` "SaveSlotName"))
  (if _returnvalue
    (bind _returnvalue_2 (`GameplayStatics.LoadGameFromSlot` "SaveSlotName"))
    (bind _assg_best_times (cast `/Game/00-Blueprints/SG_BestTimes` _returnvalue_2))
    (set `self.BestTime` (`/Game/00-Blueprints/SG_BestTimes.BestTime1` _assg_best_times))
    (else
      (set `self.BestTime` -1.0))))

(fn `Save Best Time`
  (bind _returnvalue (`GameplayStatics.CreateSaveGameObject` "/Game/00-Blueprints/SG_BestTimes.SG_BestTimes_C"))
  (set `/Game/00-Blueprints/SG_BestTimes.BestTime1` (`self.BestTime`) _returnvalue)
  (`GameplayStatics.SaveGameToSlot` _returnvalue "SaveSlotName"))

(fn `UserConstructionScript`)